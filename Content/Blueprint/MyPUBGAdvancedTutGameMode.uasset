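; PUBG-style game mode that spawns randomized loot at BeginPlay, one ItemGroup per DT_ItemGroupLocation row.
; Per group, it rolls an item count, distinct types and IDs from DataTables, mostly weighted by repeating entries in shuffled arrays.
; A rolled weapon adds its matching ammo and drops the first non-weapon entry.
; Pickups spawn at random group transforms with GameInstance serial numbers; an already-used pick reuses the previous location without retrying.
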(event `self.ReceiveBeginPlay`
  (set `self.GaimeInstanceRef` (cast `/Game/Blueprint/BP_PUBGAdvancedTutGI` (`GameplayStatics.GetGameInstance`) :!pure true))
  (`self.GenerateItems`))

(fn `GenerateItems`
  (locals (ItemGroupRef :type "/Game/Blueprint/Items/ItemGroup Object Reference") (ItemsTypeArr :type "Array of E_ItemType Enum") (ItemsIdArr :type "Array of /Game/Blueprint/Datas/ItemGeneration/STR_ItemsTypenID Structure") (SpawnType :type "E_ItemType Enum") (SpawnID :type Name) (UsedLocations :type "Array of Transform Structure") (SpawnLocation :type "Transform Structure") (ItemsObject :type "Array of PickupBase Object Reference"))
  (bind _outrownames (`DataTableFunctionLibrary.GetDataTableRowNames` "/Game/Blueprint/Datas/ItemGeneration/DT_ItemGroupLocation.DT_ItemGroupLocation"))
  (for _array_element _outrownames
    (bind _returnvalue (`|GetDataTableRow` "/Game/Blueprint/Datas/ItemGeneration/DT_ItemGroupLocation.DT_ItemGroupLocation" _array_element)
      (:`then`
        (bind _returnvalue_2 (`|SpawnActorFromClass` "/Game/Blueprint/Items/ItemGroup.ItemGroup_C" (`KismetMathLibrary.MakeTransform` (`.Location_2_4929C24C924DD254DF6E088ADBD6A55C` (break `/Game/Blueprint/Datas/TableStructures/STR_ItemGroupLocation` _returnvalue))) "Undefined" "OverrideRootScale" null null))
        (set `local.ItemGroupRef` _returnvalue_2)
        (bind _number (`self.RandomItemNumber`))
        (for _ (range (+ _number 1))
          (bind _itemtype (`self.RandomItemType` :!label _label))
          (if (== (`KismetArrayLibrary.Array_Find` (`local.ItemsTypeArr`) _itemtype) -1)
            (`KismetArrayLibrary.Array_Add` (`local.ItemsTypeArr`) _itemtype)
            (else
              (goto _label))))
        (for _array_element_2 (`local.ItemsTypeArr`)
          (bind _item (`self.RandomItemID` _array_element_2))
          (`KismetArrayLibrary.Array_Add` (`local.ItemsIdArr`) _item))
        (`KismetArrayLibrary.Array_Clear` (`local.ItemsTypeArr`))
        (for _array_element_3 (`local.ItemsIdArr`)
          (bind (_type _id) (break `/Game/Blueprint/Datas/ItemGeneration/STR_ItemsTypenID` _array_element_3))
          (if (`|EnumEquality` _type "EIT_Weapon")
            (bind _returnvalue_3 (`|GetDataTableRow` "/Game/Blueprint/Datas/DataTable/DT_ItemWeapon.DT_ItemWeapon" _id)
              (:`then`
                (`KismetArrayLibrary.Array_Add` (`local.ItemsIdArr`) (make `/Game/Blueprint/Datas/ItemGeneration/STR_ItemsTypenID` "EIT_Ammo" (`.UseAmmoID` (break `STR_ItemWeapon` _returnvalue_3))))
                (for (_array_element_4 _array_index) (`local.ItemsIdArr`)
                  (if (`|EnumInequality` (`.Type_2_5E5F0B1B8E416144476433B5DF5FDF2E` (break `/Game/Blueprint/Datas/ItemGeneration/STR_ItemsTypenID` _array_element_4)) "EIT_Weapon")
                    (`KismetArrayLibrary.Array_Remove` (`local.ItemsIdArr`) _array_index)
                    (break)))))))
        (for _array_element_5 (`local.ItemsIdArr`)
          (bind (_type_2 _id_2) (break `/Game/Blueprint/Datas/ItemGeneration/STR_ItemsTypenID` _array_element_5))
          (set `local.SpawnType` _type_2)
          (set `local.SpawnID` _id_2)
          (`|ExecutionSequence`
            (:`then_0`
              (bind _location (`self.RandomLocation` (`/Game/Blueprint/Items/ItemGroup.GetAllTransform` (`local.ItemGroupRef`))))
              (if (== (`KismetArrayLibrary.Array_Find` (`local.UsedLocations`) _location) -1)
                (bind _output_get (set `local.SpawnLocation` _location))
                (`KismetArrayLibrary.Array_Add` (`local.UsedLocations`) _output_get)))
            (:`then_1`
              (switch `E_ItemType` (`local.SpawnType`)
                (:`EIT_Weapon`
                  (bind _returnvalue_4 (`|SpawnActorFromClass` "/Script/PUBGAdvancedTut.PickupWeapon" (`local.SpawnLocation`) "Undefined" "OverrideRootScale" null 0 (`local.SpawnID`) (`/Game/Blueprint/BP_PUBGAdvancedTutGI.GenerateSN` (`self.GaimeInstanceRef`)) 1 null))
                  (`KismetArrayLibrary.Array_Add` (`local.ItemsObject`) _returnvalue_4))
                (:`EIT_Accessories`
                  (bind _returnvalue_5 (`|SpawnActorFromClass` "/Script/PUBGAdvancedTut.PickupWeaponAcc" (`local.SpawnLocation`) "Undefined" "OverrideRootScale" null (`local.SpawnID`) (`/Game/Blueprint/BP_PUBGAdvancedTutGI.GenerateSN` (`self.GaimeInstanceRef`)) 1 null))
                  (`KismetArrayLibrary.Array_Add` (`local.ItemsObject`) _returnvalue_5))
                (:`EIT_Ammo`
                  (bind _returnvalue_6 (`|SpawnActorFromClass` "/Script/PUBGAdvancedTut.PickupAmmo" (`local.SpawnLocation`) "Undefined" "OverrideRootScale" null (`local.SpawnID`) (`/Game/Blueprint/BP_PUBGAdvancedTutGI.GenerateSN` (`self.GaimeInstanceRef`)) 0 null))
                  (`KismetArrayLibrary.Array_Add` (`local.ItemsObject`) _returnvalue_6))
                (:`EIT_Health`
                  (bind _returnvalue_7 (`|SpawnActorFromClass` "/Script/PUBGAdvancedTut.PickupHealth" (`local.SpawnLocation`) "Undefined" "OverrideRootScale" null (`local.SpawnID`) (`/Game/Blueprint/BP_PUBGAdvancedTutGI.GenerateSN` (`self.GaimeInstanceRef`)) 1 null))
                  (`KismetArrayLibrary.Array_Add` (`local.ItemsObject`) _returnvalue_7))
                (:`EIT_Boost`
                  (bind _returnvalue_8 (`|SpawnActorFromClass` "/Script/PUBGAdvancedTut.PickupBoost" (`local.SpawnLocation`) "Undefined" "OverrideRootScale" null (`local.SpawnID`) (`/Game/Blueprint/BP_PUBGAdvancedTutGI.GenerateSN` (`self.GaimeInstanceRef`)) 1 null))
                  (`KismetArrayLibrary.Array_Add` (`local.ItemsObject`) _returnvalue_8))
                (:`EIT_Helmet`
                  (bind _returnvalue_9 (`|SpawnActorFromClass` "/Script/PUBGAdvancedTut.PickupEquipment" (`local.SpawnLocation`) "Undefined" "OverrideRootScale" null (`local.SpawnID`) (`/Game/Blueprint/BP_PUBGAdvancedTutGI.GenerateSN` (`self.GaimeInstanceRef`)) 1 null :!label _label_2))
                  (`KismetArrayLibrary.Array_Add` (`local.ItemsObject`) _returnvalue_9))
                (:`EIT_Vest`
                  (goto _label_2))
                (:`EIT_Backpack`
                  (goto _label_2))))))
        (`KismetArrayLibrary.Array_Clear` (`local.ItemsIdArr`))))))

(fn `RandomItemID`
  (params (ItemType :type "E_ItemType Enum" :default "EIT_Weapon"))
  (returns (Item :type "/Game/Blueprint/Datas/ItemGeneration/STR_ItemsTypenID Structure"))
  (locals (Arr :type "Array of /Game/Blueprint/Datas/ItemGeneration/STR_ItemsTypenID Structure"))
  (bind _arr (`local.Arr`))
  (`|ExecutionSequence`
    (:`then_0`
      (switch `E_ItemType` ItemType
        (:`EIT_Weapon`
          (bind _outrownames (`DataTableFunctionLibrary.GetDataTableRowNames` "/Game/Blueprint/Datas/DataTable/DT_ItemWeapon.DT_ItemWeapon"))
          (for _array_element _outrownames
            (bind _returnvalue (`|GetDataTableRow` "/Game/Blueprint/Datas/DataTable/DT_ItemWeapon.DT_ItemWeapon" _array_element)
              (:`then`
                (for _ (range (+ (`.ProbabilityPercent` (break `STR_ItemWeapon` _returnvalue)) 1))
                  (`KismetArrayLibrary.Array_Add` (`local.Arr`) (make `/Game/Blueprint/Datas/ItemGeneration/STR_ItemsTypenID` "EIT_Weapon" _array_element)))))))
        (:`EIT_Accessories`
          (bind _outrownames_2 (`DataTableFunctionLibrary.GetDataTableRowNames` "/Game/Blueprint/Datas/DataTable/DT_ItemWeaponAcc.DT_ItemWeaponAcc"))
          (for _array_element_2 _outrownames_2
            (`KismetArrayLibrary.Array_Add` (`local.Arr`) (make `/Game/Blueprint/Datas/ItemGeneration/STR_ItemsTypenID` "EIT_Accessories" _array_element_2))))
        (:`EIT_Ammo`
          (bind _outrownames_3 (`DataTableFunctionLibrary.GetDataTableRowNames` "/Game/Blueprint/Datas/DataTable/DT_ItemAmmo.DT_ItemAmmo"))
          (for _array_element_3 _outrownames_3
            (bind _returnvalue_2 (`|GetDataTableRow` "/Game/Blueprint/Datas/DataTable/DT_ItemAmmo.DT_ItemAmmo" _array_element_3)
              (:`then`
                (for _ (range (+ (`.ProbabilityPercent` (break `STR_ItemAmmo` _returnvalue_2)) 1))
                  (`KismetArrayLibrary.Array_Add` (`local.Arr`) (make `/Game/Blueprint/Datas/ItemGeneration/STR_ItemsTypenID` "EIT_Ammo" _array_element_3)))))))
        (:`EIT_Health`
          (bind _outrownames_4 (`DataTableFunctionLibrary.GetDataTableRowNames` "/Game/Blueprint/Datas/DataTable/DT_ItemHealth.DT_ItemHealth"))
          (for _array_element_4 _outrownames_4
            (bind _returnvalue_3 (`|GetDataTableRow` "/Game/Blueprint/Datas/DataTable/DT_ItemHealth.DT_ItemHealth" _array_element_4)
              (:`then`
                (for _ (range (+ (`.ProbabilityPercent` (break `STR_ItemHealth` _returnvalue_3)) 1))
                  (`KismetArrayLibrary.Array_Add` (`local.Arr`) (make `/Game/Blueprint/Datas/ItemGeneration/STR_ItemsTypenID` "EIT_Health" _array_element_4)))))))
        (:`EIT_Boost`
          (bind _outrownames_5 (`DataTableFunctionLibrary.GetDataTableRowNames` "/Game/Blueprint/Datas/DataTable/DT_ItemBoost.DT_ItemBoost"))
          (for _array_element_5 _outrownames_5
            (bind _returnvalue_4 (`|GetDataTableRow` "/Game/Blueprint/Datas/DataTable/DT_ItemBoost.DT_ItemBoost" _array_element_5)
              (:`then`
                (for _ (range (+ (`.ProbabilityPercent` (break `STR_ItemBoost` _returnvalue_4)) 1))
                  (`KismetArrayLibrary.Array_Add` (`local.Arr`) (make `/Game/Blueprint/Datas/ItemGeneration/STR_ItemsTypenID` "EIT_Boost" _array_element_5)))))))
        (:`EIT_Helmet`
          (bind _outrownames_6 (`DataTableFunctionLibrary.GetDataTableRowNames` "/Game/Blueprint/Datas/DataTable/DT_ItemEquipment.DT_ItemEquipment"))
          (for _array_element_6 _outrownames_6
            (bind _returnvalue_5 (`|GetDataTableRow` "/Game/Blueprint/Datas/DataTable/DT_ItemEquipment.DT_ItemEquipment" _array_element_6)
              (:`then`
                (bind (_name _type _pickupmesh _icon _thumbnails _capacity _probabilitypercent) (break `STR_ItemEquipment` _returnvalue_5))
                (if (`|EnumEquality` _type "EIT_Helmet")
                  (for _ (range (+ _probabilitypercent 1))
                    (`KismetArrayLibrary.Array_Add` (`local.Arr`) (make `/Game/Blueprint/Datas/ItemGeneration/STR_ItemsTypenID` "EIT_Helmet" _array_element_6))))))))
        (:`EIT_Vest`
          (bind _outrownames_7 (`DataTableFunctionLibrary.GetDataTableRowNames` "/Game/Blueprint/Datas/DataTable/DT_ItemEquipment.DT_ItemEquipment"))
          (for _array_element_7 _outrownames_7
            (bind _returnvalue_6 (`|GetDataTableRow` "/Game/Blueprint/Datas/DataTable/DT_ItemEquipment.DT_ItemEquipment" _array_element_7)
              (:`then`
                (bind (_name_2 _type_2 _pickupmesh_2 _icon_2 _thumbnails_2 _capacity_2 _probabilitypercent_2) (break `STR_ItemEquipment` _returnvalue_6))
                (if (`|EnumEquality` _type_2 "EIT_Vest")
                  (for _ (range (+ _probabilitypercent_2 1))
                    (`KismetArrayLibrary.Array_Add` (`local.Arr`) (make `/Game/Blueprint/Datas/ItemGeneration/STR_ItemsTypenID` "EIT_Vest" _array_element_7))))))))
        (:`EIT_Backpack`
          (bind _outrownames_8 (`DataTableFunctionLibrary.GetDataTableRowNames` "/Game/Blueprint/Datas/DataTable/DT_ItemEquipment.DT_ItemEquipment"))
          (for _array_element_8 _outrownames_8
            (bind _returnvalue_7 (`|GetDataTableRow` "/Game/Blueprint/Datas/DataTable/DT_ItemEquipment.DT_ItemEquipment" _array_element_8)
              (:`then`
                (bind (_name_3 _type_3 _pickupmesh_3 _icon_3 _thumbnails_3 _capacity_3 _probabilitypercent_3) (break `STR_ItemEquipment` _returnvalue_7))
                (if (`|EnumEquality` _type_3 "EIT_Backpack")
                  (for _ (range (+ _probabilitypercent_3 1))
                    (`KismetArrayLibrary.Array_Add` (`local.Arr`) (make `/Game/Blueprint/Datas/ItemGeneration/STR_ItemsTypenID` "EIT_Backpack" _array_element_8))))))))))
    (:`then_1`
      (`KismetArrayLibrary.Array_Shuffle` _arr)
      (return (`|GetArrayItem` _arr (`KismetMathLibrary.RandomIntegerInRange` 0 (- (`KismetArrayLibrary.Array_Length` (`local.Arr`)) 1)))))))

(fn `RandomItemNumber`
  (returns (Number :type Integer))
  (locals (Arr :type "Array of Integer"))
  (bind _arr (`local.Arr`))
  (bind _outrownames (`DataTableFunctionLibrary.GetDataTableRowNames` "/Game/Blueprint/Datas/ItemGeneration/DT_NumberProbability.DT_NumberProbability"))
  (for _array_element _outrownames
    (bind _returnvalue (`|GetDataTableRow` "/Game/Blueprint/Datas/ItemGeneration/DT_NumberProbability.DT_NumberProbability" _array_element)
      (:`then`
        (bind (_percentage _number) (break `STR_NumberProbability` _returnvalue))
        (for _ (range (+ _percentage 1))
          (`KismetArrayLibrary.Array_Add` (`local.Arr`) _number)))))
  (`KismetArrayLibrary.Array_Shuffle` _arr)
  (return (`|GetArrayItem` _arr (`KismetMathLibrary.RandomIntegerInRange` 0 99))))

(fn `RandomItemType`
  (returns (ItemType :type "E_ItemType Enum"))
  (locals (Arr :type "Array of E_ItemType Enum"))
  (bind _arr (`local.Arr`))
  (bind _outrownames (`DataTableFunctionLibrary.GetDataTableRowNames` "/Game/Blueprint/Datas/ItemGeneration/DT_ItemTypeProbability.DT_ItemTypeProbability"))
  (for _array_element _outrownames
    (bind _returnvalue (`|GetDataTableRow` "/Game/Blueprint/Datas/ItemGeneration/DT_ItemTypeProbability.DT_ItemTypeProbability" _array_element)
      (:`then`
        (bind (_percentage _type) (break `STR_ItemTypeProbability` _returnvalue))
        (for _ (range 1 (+ _percentage 1))
          (`KismetArrayLibrary.Array_Add` (`local.Arr`) _type)))))
  (`KismetArrayLibrary.Array_Shuffle` _arr)
  (return (`|GetArrayItem` _arr (`KismetMathLibrary.RandomIntegerInRange` 0 99))))

(fn `RandomLocation`
  (params (Available :type "Array of Transform Structure"))
  (returns (Location :type "Transform Structure"))
  (return (`|GetArrayItem` Available (`KismetMathLibrary.RandomIntegerInRange` 0 (- (`KismetArrayLibrary.Array_Length` Available) 1)))))

(fn `UserConstructionScript`)