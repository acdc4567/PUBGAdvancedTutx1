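; Game mode Blueprint for a PUBG-style tutorial project that handles item spawn points and item count odds.
; GenerateItems spawns an ItemGroup actor at each location listed in DT_ItemGroupLocation.
; RandomItemNumber expands DT_NumberProbability percentages into a shuffled weighted array, then tallies occurrences of 3, 4 and 5.
; Its random-pick return is disconnected, and neither function calls the other.
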(fn `GenerateItems`
  (locals (ItemGroupRef :type "/Game/Blueprint/Items/ItemGroup Object Reference"))
  (bind _outrownames (`DataTableFunctionLibrary.GetDataTableRowNames` "/Game/Blueprint/Datas/ItemGeneration/DT_ItemGroupLocation.DT_ItemGroupLocation"))
  (for _array_element _outrownames
    (bind _returnvalue (`|GetDataTableRow` "/Game/Blueprint/Datas/ItemGeneration/DT_ItemGroupLocation.DT_ItemGroupLocation" _array_element)
      (:`then`
        (bind _returnvalue_2 (`|SpawnActorFromClass` "/Game/Blueprint/Items/ItemGroup.ItemGroup_C" (`KismetMathLibrary.MakeTransform` (`.Location_2_4929C24C924DD254DF6E088ADBD6A55C` (break `/Game/Blueprint/Datas/TableStructures/STR_ItemGroupLocation` _returnvalue))) "Undefined" "OverrideRootScale" null null))
        (set `local.ItemGroupRef` _returnvalue_2)))))

(fn `RandomItemNumber`
  (returns (Number :type Integer))
  (locals (Arr :type "Array of Integer") (`3` :type Integer) (`4` :type Integer) (`5` :type Integer))
  (bind _arr (`local.Arr`))
  (bind _outrownames (`DataTableFunctionLibrary.GetDataTableRowNames` "/Game/Blueprint/Datas/ItemGeneration/DT_NumberProbability.DT_NumberProbability"))
  (for _array_element _outrownames
    (bind _returnvalue (`|GetDataTableRow` "/Game/Blueprint/Datas/ItemGeneration/DT_NumberProbability.DT_NumberProbability" _array_element)
      (:`then`
        (bind (_percentage _number) (break `STR_NumberProbability` _returnvalue))
        (for _ (range (+ _percentage 1))
          (`KismetArrayLibrary.Array_Add` (`local.Arr`) _number)))))
  (`KismetArrayLibrary.Array_Shuffle` _arr)
  (for _array_element_2 _arr
    (if (== _array_element_2 3)
      (`/Engine/EditorBlueprintResources/StandardMacros.IncrementInt` (`local.3`))
      (elif (== _array_element_2 4)
        (`/Engine/EditorBlueprintResources/StandardMacros.IncrementInt` (`local.4`))
        (elif (== _array_element_2 5)
          (`/Engine/EditorBlueprintResources/StandardMacros.IncrementInt` (`local.5`)))))))

(fn `UserConstructionScript`)