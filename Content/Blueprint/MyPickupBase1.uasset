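; MyPickupBase1 is a pickup actor, apparently a base class, that sets its height at spawn and can be outlined.
; On BeginPlay it line traces downward for one object type and moves itself a fixed height above the hit, without checking that the trace hit.
; EnabledOutline toggles custom depth rendering on the static mesh, presumably for a post-process highlight.
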(event `self.ReceiveBeginPlay`
  (bind (_returnvalue_x _returnvalue_y _returnvalue_z) (`KismetMathLibrary.BreakVector` (`self.K2_GetActorLocation`)))
  (`parent.ReceiveBeginPlay`)
  (bind _outhit (`KismetSystemLibrary.LineTraceSingleForObjects` (`self.K2_GetActorLocation`) (`KismetMathLibrary.MakeVector` _returnvalue_x _returnvalue_y (+ _returnvalue_z -1000.0)) (`|MakeArray` "ObjectTypeQuery7" :!type "EObjectTypeQuery Enum")))
  (`self.K2_SetActorLocation` (`KismetMathLibrary.MakeVector` _returnvalue_x _returnvalue_y (+ (.z (`.Location` (`GameplayStatics.BreakHitResult` _outhit))) 200.0))))

(fn `EnabledOutline`
  (params (bEnabled :type Boolean))
  (bind _staticmesh (`self.StaticMesh`))
  (if bEnabled
    (`PrimitiveComponent.SetRenderCustomDepth` _staticmesh true)
    (else
      (`PrimitiveComponent.SetRenderCustomDepth` _staticmesh false))))

(fn `UserConstructionScript`)