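; Player controller for a PUBG-style game that keeps the character's visible weapons and equipment in sync with the player state.
; On BeginPlay it caches the character, game instance and player state, then binds to the player state's weapon-changed and equipment-changed delegates.
; Weapon changes refresh the weapon display using the character's calculated hold-gun socket.
; Equipment changes refresh both equipment and weapon displays, passing "None" as the socket.
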(event `self.ReceiveBeginPlay`
  (`|ExecutionSequence`
    (:`then_0`
      (set `self.MyCharacterRef` (cast `/Game/Character/MyCharacter` (`GameplayStatics.GetPlayerCharacter` 0) :!pure true))
      (set `self.MyGameInstanceRef` (cast `/Game/Blueprint/BP_PUBGAdvancedTutGI` (`GameplayStatics.GetGameInstance`) :!pure true))
      (set `self.MyPlayerStateRef` (cast `SPlayerState` (`self.PlayerState`) :!pure true)))
    (:`then_1`
      (add `SPlayerState.OnWeaponChanged` (`self.MyPlayerStateRef`) (delegate `OnWeaponChanged_Event_0`))
      (add `SPlayerState.OnEquipmentChanged` (`self.MyPlayerStateRef`) (delegate `OnEquipmentChanged_Event_0`)))))

(event `OnWeaponChanged_Event_0`
  (params (Weapon :type "ItemWeapon Object Reference") (Position :type "E_WeaponPosition Enum" :default "EWP_Left") (bIsOnHand :type Boolean))
  (bind _mycharacterref (`self.MyCharacterRef`))
  (`SCharacter.UpdateWeaponDisplay` _mycharacterref (`SCharacter.CalculateHoldGunSocket` _mycharacterref)))

(event `OnEquipmentChanged_Event_0`
  (params (Equipment :type "ItemBase Object Reference") (bIsAdd :type Boolean))
  (bind _mycharacterref (`self.MyCharacterRef`))
  (`SCharacter.UpdateEquipmentDisplay` _mycharacterref)
  (`SCharacter.UpdateWeaponDisplay` _mycharacterref "None"))

(fn `UserConstructionScript`)