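; ItemGroup is an item Blueprint that acts as a layout template for a group of five static mesh components.
; GetAllTransform returns the world transforms of those five meshes as an array.
; The construction script is empty, and the file holds no other logic.
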(fn `GetAllTransform`
  (returns (Transforms :type "Array of Transform Structure"))
  (return (`|MakeArray` (`SceneComponent.K2_GetComponentToWorld` (`self.StaticMesh`)) (`SceneComponent.K2_GetComponentToWorld` (`self.StaticMesh1`)) (`SceneComponent.K2_GetComponentToWorld` (`self.StaticMesh2`)) (`SceneComponent.K2_GetComponentToWorld` (`self.StaticMesh3`)) (`SceneComponent.K2_GetComponentToWorld` (`self.StaticMesh4`)))))

(fn `UserConstructionScript`)